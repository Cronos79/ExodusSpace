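; BP_ESAICharacter is an AI character Blueprint that gives visual feedback for damage and death.
; It reacts to the attribute component's health-change event and checks whether the character is still alive.
; Non-positive changes while alive stamp the current time into a material scalar parameter, presumably driving a time-based hit flash.
; On death, it applies a red-tinted dynamic test material, disables movement and sets a short lifespan so the actor destroys itself.
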(event OnHealthChanged(AttributeComp)
  (params (InstigatorActor :type Actor%20Object%20Reference) (OwningComp :type Cro%20Attribute%20Component%20Object%20Reference) (NewHealth :type Float%20%28single-precision%29) (MaxHealth :type Float%20%28single-precision%29) (ChangedAmount :type Float%20%28single-precision%29))
  (bind _returnvalue (Class|CroAttributeComponent|IsAlive (Variables|Default|GetAttributeComp)))
  (if _returnvalue
    (if (<= ChangedAmount 0.0)
      (Rendering|Material|SetScalarParameterValueonMaterials (Variables|Default|GetTempChar) "TimeToHit" (Utilities|Time|GetTimeSeconds)))
    (else
      (bind _returnvalue_2 (Rendering|Material|CreateDynamicMaterialInstance (Variables|Default|GetTempChar) 0 "/Game/Materials/M_TestMat.M_TestMat" "None" :!class /Script/Engine.PrimitiveComponent))
      (Rendering|Material|SetVectorParameterValue _returnvalue_2 "Color" "(R=1.000000,G=0.000000,B=0.000000,A=1.000000)" :!class /Script/Engine.MaterialInstanceDynamic)
      (Actor|SetLifeSpan 2.0)
      (Pawn|Components|CharacterMovement|DisableMovement (Variables|Character|GetCharacterMovement)))))

(fn ConstructionScript)