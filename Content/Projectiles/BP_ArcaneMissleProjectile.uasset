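; BP_ArcaneMissleProjectile is a projectile that damages the first non-instigator actor it overlaps.
; An overlapped actor whose action component carries the parry tag instead reflects it, reversing velocity and, if a pawn, becoming the new instigator.
; On a hit it activates impact FX, hides the missile FX, disables collision, applies damage credited to the instigator and expires after a short lifespan.
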(event OnComponentBeginOverlap(SphereComp)
  (params (OverlappedComponent :type Primitive%20Component%20Object%20Reference) (OtherActor :type Actor%20Object%20Reference) (OtherComp :type Primitive%20Component%20Object%20Reference) (OtherBodyIndex :type Integer) (bFromSweep :type Boolean) (SweepResult :type Hit%20Result%20Structure%20%28by%20ref%29))
  (bind _returnvalue (Actor|GetComponentbyClass OtherActor "/Script/CroAction.CroActionComponent"))
  (bind _movecomp (Variables|Default|GetMoveComp))
  (Utilities|IsValid _returnvalue
    (:Is%20Valid
      (if (GameplayTags|HasTag (Variables|/Script/CroAction.CroActionComponent|GetActiveGameplayTags _returnvalue) (Variables|Default|GetParryTag))
        (Variables|/Script/Engine.MovementComponent|SetVelocity _movecomp (* (Variables|/Script/Engine.MovementComponent|GetVelocity _movecomp) -1))
        (bind _aspawn (Utilities|Casting|CastToPawn OtherActor))
        (Variables|Default|SetInstigator _aspawn)
        (else
          (if (!= OtherActor (Variables|Default|GetInstigator)) :!label _label
            (Class|ESProjectileBase|OnHit OtherActor)))))
    (:Is%20Not%20Valid
      (goto _label))))

(event EventOnHit
  (params (HitActor :type Actor%20Object%20Reference))
  (bind _instigator (Variables|Default|GetInstigator))
  (Components|Activation|Activate (Variables|Default|GetHitFX) false)
  (Actor|SetLifeSpan 1.5)
  (Collision|SetCollisionEnabled (Variables|Default|GetSphereComp) "NoCollision")
  (Rendering|SetVisibility (Variables|Default|GetMissleFX) false false)
  (Game|Damage|ApplyDamage HitActor (Variables|Default|GetDamage) (Game|GetInstigatorController _instigator) _instigator))

(fn ConstructionScript)